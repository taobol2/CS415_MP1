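; BP_Tunnel is an endless-tunnel segment with a rotating holed wall the player must pass through.
; Overlapping its box makes TunnelSpawner add a tunnel, destroys this one, increments score and randomly spawns health packs and enemies ahead.
; Hitting the wall shakes the camera, then either triggers death and restart or nudges the player forward with collision disabled, reducing health and score.
; RandomizeWall picks a random hole mesh and roll.
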(event OnComponentBeginOverlap(BoxExtent)
  (params (OverlappedComponent :type Primitive%20Component%20Object%20Reference) (OtherActor :type Actor%20Object%20Reference) (OtherComp :type Primitive%20Component%20Object%20Reference) (OtherBodyIndex :type Integer) (bFromSweep :type Boolean) (SweepResult :type Hit%20Result%20Structure%20%28by%20ref%29))
  (bind _asbp_player (Utilities|Casting|CastToBP_Player OtherActor))
  (Utilities|FlowControl|Sequence
    (:then_0
      (Default|SpawnTunnelatSpawnPoint (Variables|Default|GetTunnelSpawner))
      (Actor|DestroyActor))
    (:then_1
      (Variables|/Game/InfiniteMatrix/Blueprints/BP_Player.BP_Player_C|SetScore _asbp_player (+ (Variables|/Game/InfiniteMatrix/Blueprints/BP_Player.BP_Player_C|GetScore _asbp_player) 1)))
    (:then_2
      (CallFunction|SpawnHealthPack))
    (:then_3
      (CallFunction|SpawnEnemies))))

(event OnComponentHit(WallMesh)
  (params (HitComponent :type Primitive%20Component%20Object%20Reference) (OtherActor :type Actor%20Object%20Reference) (OtherComp :type Primitive%20Component%20Object%20Reference) (NormalImpulse :type Vector :default "0, 0, 0") (Hit :type Hit%20Result%20Structure%20%28by%20ref%29))
  (Development|PrintString "AAA")
  (bind _asbp_player (Utilities|Casting|CastToBP_Player OtherActor))
  (Camera|PlayWorldCameraShake "/Game/InfiniteMatrix/Blueprints/BP_CameraShake.BP_CameraShake_C" (Transformation|GetActorLocation _asbp_player) 0.0 3e+03)
  (if (<= (- (Variables|/Game/InfiniteMatrix/Blueprints/BP_Player.BP_Player_C|GetHealth _asbp_player) (Variables|Default|GetDamageVal)) 0.0)
    (Variables|/Game/InfiniteMatrix/Blueprints/BP_Player.BP_Player_C|SetHealth _asbp_player 0.0)
    (Variables|/Game/InfiniteMatrix/Blueprints/BP_Player.BP_Player_C|SetIsDead _asbp_player true)
    (Default|DisplayRestart _asbp_player)
    (else
      (Utilities|FlowControl|Sequence
        (:then_0
          (Collision|SetActorEnableCollision _asbp_player false))
        (:then_1
          (Transformation|SetActorLocation _asbp_player (Math|Vector|MakeVector (+ (.x (Transformation|GetActorLocation _asbp_player)) 6e+01) (.y (Transformation|GetActorLocation _asbp_player)) (.z (Transformation|GetActorLocation _asbp_player))) true false))
        (:then_2
          (Collision|SetActorEnableCollision _asbp_player true))
        (:then_3
          (Variables|/Game/InfiniteMatrix/Blueprints/BP_Player.BP_Player_C|SetHealth _asbp_player (- (Variables|/Game/InfiniteMatrix/Blueprints/BP_Player.BP_Player_C|GetHealth _asbp_player) (Variables|Default|GetDamageVal))))
        (:then_4
          (Variables|/Game/InfiniteMatrix/Blueprints/BP_Player.BP_Player_C|SetScore _asbp_player (- (Variables|/Game/InfiniteMatrix/Blueprints/BP_Player.BP_Player_C|GetScore _asbp_player) 1)))))))

(event EventBeginPlay)

(event EventTick
  (params (DeltaSeconds :type Float%20%28single-precision%29))
  (Transformation|AddLocalRotation (Variables|Default|GetWallMesh) (Math|Rotator|MakeRotator (* DeltaSeconds (Variables|Default|GetRotateSpeed)) 0.0 0.0) false false))

(fn ConstructionScript)

(fn RandomizeWall
  (Components|StaticMesh|SetStaticMesh (Variables|Default|GetWallMesh) (Utilities|Select :Index (Math|Random|RandomIntegerinRange 0 3) :Option%200 "/Game/InfiniteMatrix/Meshes/SM_Hole_01.SM_Hole_01" :Option%201 "/Game/InfiniteMatrix/Meshes/SM_Hole_02.SM_Hole_02" :Option%202 "/Game/InfiniteMatrix/Meshes/SM_Hole_03.SM_Hole_03" :Option%203 "/Game/InfiniteMatrix/Meshes/SM_Hole_04.SM_Hole_04"))
  (Transformation|AddLocalRotation (Variables|Default|GetWallMesh) (Math|Rotator|MakeRotator (Math|Random|RandomFloatinRange 0.0 3.6e+02) 0.0 0.0) false false))

(fn SpawnHealthPack
  (bind _returnvalue (Game|Player|GetPlayerPawn 0))
  (bind _returnvalue_2 (Transformation|GetActorLocation _returnvalue))
  (if (<= (Math|Random|RandomFloatinRange 0.0 1.0) 0.5)
    (Game|SpawnActorfromClass "/Game/InfiniteMatrix/Blueprints/BP_Health.BP_Health_C" (Math|Transform|MakeTransform (Math|Vector|MakeVector (+ (.x _returnvalue_2) (Math|Random|RandomFloatinRange 5e+02 2e+03)) (+ (.y _returnvalue_2) (Math|Random|RandomFloatinRange -1e+02 1e+02)) (+ (.z _returnvalue_2) (Math|Random|RandomFloatinRange -1e+02 1e+02))) "0, 0, 0" "1.000000,1.000000,1.000000") "Undefined" "MultiplyWithRoot" 0 0)))

(fn SpawnEnemies
  (bind _returnvalue (Game|Player|GetPlayerPawn 0))
  (bind _returnvalue_2 (Transformation|GetActorLocation _returnvalue))
  (if (<= (Math|Random|RandomFloatinRange 0.0 1.0) 0.5)
    (Game|SpawnActorfromClass "/Game/InfiniteMatrix/Blueprints/BP_Enemies.BP_Enemies_C" (Math|Transform|MakeTransform (Math|Vector|MakeVector (+ (.x _returnvalue_2) (Math|Random|RandomFloatinRange 1e+03 2e+03)) (+ (.y _returnvalue_2) (Math|Random|RandomFloatinRange -1e+02 1e+02)) (+ (.z _returnvalue_2) (Math|Random|RandomFloatinRange -1e+02 1e+02))) "0, 0, 0" "1.000000,1.000000,1.000000") "Undefined" "MultiplyWithRoot" 0 0)))